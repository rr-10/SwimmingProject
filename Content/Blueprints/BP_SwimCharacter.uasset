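; BP_SwimCharacter is a character that switches between walking and swimming by depth in water, and adds the PlayerHUD widget on BeginPlay.
; EnterWater and ExitWater set the InWater flag, with entry also recording the actor's Z as water level.
; Tick compares depth below that level to capsule half-height, using paired DoOnce gates to toggle movement mode and the physics volume's WaterVolume flag.
; The shallow-side threshold divides half-height by zero.
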(event `self.ReceiveBeginPlay`
  (bind _returnvalue (`GameplayStatics.GetPlayerController` 0))
  (bind _returnvalue_2 (`|CreateWidget` "/Game/UI/PlayerHUD.PlayerHUD_C" _returnvalue))
  (`UserWidget.AddToViewport` _returnvalue_2 0)
  (`WidgetBlueprintLibrary.SetInputMode_GameOnly` _returnvalue))

(event `self.ReceiveTick`
  (params (DeltaSeconds :type "Float (single-precision)"))
  (bind (_returnvalue_x _returnvalue_y _returnvalue_z) (`KismetMathLibrary.BreakVector` (`self.K2_GetActorLocation`)))
  (bind _waterz (`self.WaterZ`))
  (bind _charactermovement (`self.CharacterMovement`))
  (bind _capsulehalfheight (`CapsuleComponent.CapsuleHalfHeight` (`self.CapsuleComponent`)))
  (if (`self.InWater`)
    (if (> (- _waterz _returnvalue_z) _capsulehalfheight)
      (`/Engine/EditorBlueprintResources/StandardMacros.DoOnce` false :!label _label
        (:`Completed`
          (set `PhysicsVolume.bWaterVolume` true (`MovementComponent.GetPhysicsVolume` _charactermovement))
          (`CharacterMovementComponent.SetMovementMode` _charactermovement "MOVE_Swimming" 0)
          (goto _label_2 :!via `Reset`)))
      (elif (< (- _waterz _returnvalue_z) (/ _capsulehalfheight 0.0))
        (`/Engine/EditorBlueprintResources/StandardMacros.DoOnce` false :!label _label_2
          (:`Completed`
            (set `PhysicsVolume.bWaterVolume` false (`MovementComponent.GetPhysicsVolume` _charactermovement))
            (`CharacterMovementComponent.SetMovementMode` _charactermovement "MOVE_Walking" 0)
            (goto _label :!via `Reset`)))))))

(event `SwimInterface.EnterWater`
  (bind (_returnvalue_x _returnvalue_y _returnvalue_z) (`KismetMathLibrary.BreakVector` (`self.K2_GetActorLocation`)))
  (set `self.InWater` true)
  (set `self.WaterZ` _returnvalue_z))

(event `SwimInterface.ExitWater`
  (set `self.InWater` false))

(fn `UserConstructionScript`)